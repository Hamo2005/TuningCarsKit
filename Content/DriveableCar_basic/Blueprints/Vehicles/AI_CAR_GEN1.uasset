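; AI-driven traffic car that follows the spline of the ROAD actor matching its lane type.
; Tick steers toward the closest spline point, while a half-second loop sets throttle against a target speed, both tuned through the game instance.
; Overlap boxes override these to reverse throttle or swerve, and a menu flag teleports the car near a respawn transform.
; Includes light, caliper and door helpers; impact sound playback is disconnected.
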(event OnComponentBeginOverlap(Box_F)
  (params (OverlappedComponent :type Primitive%20Component%20Object%20Reference) (OtherActor :type Actor%20Object%20Reference) (OtherComp :type Primitive%20Component%20Object%20Reference) (OtherBodyIndex :type Integer) (bFromSweep :type Boolean) (SweepResult :type Hit%20Result%20Structure%20%28by%20ref%29))
  (Variables|Default|SetOVERLAPPED_M true)
  (Utilities|FlowControl|Delay 0.9)
  (Variables|Default|SetOVERLAPPED_M false))

(event OnComponentEndOverlap(Box_F)
  (params (OverlappedComponent :type Primitive%20Component%20Object%20Reference) (OtherActor :type Actor%20Object%20Reference) (OtherComp :type Primitive%20Component%20Object%20Reference) (OtherBodyIndex :type Integer))
  (Variables|Default|SetOVERLAPPED_M false))

(event OnComponentHit(Mesh)
  (params (HitComponent :type Primitive%20Component%20Object%20Reference) (OtherActor :type Actor%20Object%20Reference) (OtherComp :type Primitive%20Component%20Object%20Reference) (NormalImpulse :type Vector :default "0, 0, 0") (Hit :type Hit%20Result%20Structure%20%28by%20ref%29))
  ;[0.003424 0.3159 1 0.386] impact sounds
  ;;[1 1 1] define vars
  (Variables|Impacts|SethitActor OtherActor)
  (Variables|Impacts|SetHitNormalImpulse NormalImpulse)
  (Variables|Impacts|SetHitResult Hit)
  ;;[1 1 1] checks if car hits with any player
  (bind _outactors (Actor|GetAllActorsOfClass "/Game/DriveableCar_basic/Blueprints/BP_ThirdPersonCharacter.BP_ThirdPersonCharacter_C"))
  (bind _asbp_third_person_character (Utilities|Casting|CastToBP_ThirdPersonCharacter (Variables|Impacts|GethitActor))
    (:then
      _)
    (:CastFailed
      _))
  (if (not (Utilities|Array|ContainsItem _outactors _asbp_third_person_character))
    ;;[1 1 1] is hit actor valid?
    (Utilities|IsValid (Variables|Impacts|GethitActor)
      (:Is%20Valid
        (Utilities|FlowControl|DoOnce false
          (:Completed
            ;;[1 1 1] define impact magnitude
            (Variables|Impacts|Setimpact (Math|Vector|VectorLength (- (Transformation|GetVelocity (Variables|Impacts|GethitActor)) (Transformation|GetVelocity))))
            ;;[1 1 1] checks if impact is above threshold
            (Math|Float|CompareFloat (Variables|Impacts|Getimpact) (Variables|Impacts|Getmin_impact)
              (:>)
              (:==
                _)
              (:<
                _))
            (CallFunction|CEResetDoOnceImpactSound)))))))

(event OnComponentEndOverlap(Box_R1)
  (params (OverlappedComponent :type Primitive%20Component%20Object%20Reference) (OtherActor :type Actor%20Object%20Reference) (OtherComp :type Primitive%20Component%20Object%20Reference) (OtherBodyIndex :type Integer))
  (Variables|Default|SetOVERLAPPED_S false))

(event OnComponentEndOverlap(Box_L1)
  (params (OverlappedComponent :type Primitive%20Component%20Object%20Reference) (OtherActor :type Actor%20Object%20Reference) (OtherComp :type Primitive%20Component%20Object%20Reference) (OtherBodyIndex :type Integer))
  (Variables|Default|SetOVERLAPPED_S false))

(event OnComponentBeginOverlap(Box_L1)
  (params (OverlappedComponent :type Primitive%20Component%20Object%20Reference) (OtherActor :type Actor%20Object%20Reference) (OtherComp :type Primitive%20Component%20Object%20Reference) (OtherBodyIndex :type Integer) (bFromSweep :type Boolean) (SweepResult :type Hit%20Result%20Structure%20%28by%20ref%29))
  (bind _output_get (Variables|Default|SetOverlapped%20Component%20OF%20L1 OverlappedComponent))
  (if (> (CallFunction|GetForwardSpeed) 4e+01)
    (if (not (== _output_get (Variables|Default|GetOverlapped%20Component%20OF%20R)))
      (Variables|Default|SetOVERLAPPED_S true)
      (Variables|Default|SetIS_RIGHT? false)
      (Utilities|FlowControl|Delay 0.5)
      (Variables|Default|SetOVERLAPPED_S false))))

(event OnComponentBeginOverlap(Box_F2)
  (params (OverlappedComponent :type Primitive%20Component%20Object%20Reference) (OtherActor :type Actor%20Object%20Reference) (OtherComp :type Primitive%20Component%20Object%20Reference) (OtherBodyIndex :type Integer) (bFromSweep :type Boolean) (SweepResult :type Hit%20Result%20Structure%20%28by%20ref%29))
  (Variables|Default|SetOVERLAPPED_M true))

(event OnComponentEndOverlap(Box_F2)
  (params (OverlappedComponent :type Primitive%20Component%20Object%20Reference) (OtherActor :type Actor%20Object%20Reference) (OtherComp :type Primitive%20Component%20Object%20Reference) (OtherBodyIndex :type Integer))
  (Variables|Default|SetOVERLAPPED_M false))

(event OnComponentBeginOverlap(Box_B)
  (params (OverlappedComponent :type Primitive%20Component%20Object%20Reference) (OtherActor :type Actor%20Object%20Reference) (OtherComp :type Primitive%20Component%20Object%20Reference) (OtherBodyIndex :type Integer) (bFromSweep :type Boolean) (SweepResult :type Hit%20Result%20Structure%20%28by%20ref%29))
  (Variables|Default|SetOVERLAPPED_M false))

(event OnComponentBeginOverlap(Box_F1)
  (params (OverlappedComponent :type Primitive%20Component%20Object%20Reference) (OtherActor :type Actor%20Object%20Reference) (OtherComp :type Primitive%20Component%20Object%20Reference) (OtherBodyIndex :type Integer) (bFromSweep :type Boolean) (SweepResult :type Hit%20Result%20Structure%20%28by%20ref%29))
  (if (> (CallFunction|GetForwardSpeed) 7e+01)
    (Variables|Default|SetOVERLAPPED_M true)
    (Utilities|FlowControl|Delay 0.6)
    (Variables|Default|SetOVERLAPPED_M false)))

(event OnComponentBeginOverlap(Box_R)
  (params (OverlappedComponent :type Primitive%20Component%20Object%20Reference) (OtherActor :type Actor%20Object%20Reference) (OtherComp :type Primitive%20Component%20Object%20Reference) (OtherBodyIndex :type Integer) (bFromSweep :type Boolean) (SweepResult :type Hit%20Result%20Structure%20%28by%20ref%29))
  (Variables|Default|SetOverlapped%20Component%20OF%20R OverlappedComponent)
  (Variables|Default|SetOVERLAPPED_S true)
  (Variables|Default|SetIS_RIGHT? true)
  (Utilities|FlowControl|Delay 0.8)
  (Variables|Default|SetOVERLAPPED_S false))

(event OnComponentBeginOverlap(Box_L)
  (params (OverlappedComponent :type Primitive%20Component%20Object%20Reference) (OtherActor :type Actor%20Object%20Reference) (OtherComp :type Primitive%20Component%20Object%20Reference) (OtherBodyIndex :type Integer) (bFromSweep :type Boolean) (SweepResult :type Hit%20Result%20Structure%20%28by%20ref%29))
  (Variables|Default|SetOverlapped%20Component%20OF%20L OverlappedComponent)
  (Variables|Default|SetOVERLAPPED_S true)
  (Variables|Default|SetIS_RIGHT? false)
  (Utilities|FlowControl|Delay 0.8)
  (Variables|Default|SetOVERLAPPED_S false))

(event OnComponentEndOverlap(Box_L)
  (params (OverlappedComponent :type Primitive%20Component%20Object%20Reference) (OtherActor :type Actor%20Object%20Reference) (OtherComp :type Primitive%20Component%20Object%20Reference) (OtherBodyIndex :type Integer))
  (Variables|Default|SetOVERLAPPED_S false))

(event OnComponentEndOverlap(Box_R)
  (params (OverlappedComponent :type Primitive%20Component%20Object%20Reference) (OtherActor :type Actor%20Object%20Reference) (OtherComp :type Primitive%20Component%20Object%20Reference) (OtherBodyIndex :type Integer))
  (Variables|Default|SetOVERLAPPED_S false))

(event OnComponentEndOverlap(Box_F1)
  (params (OverlappedComponent :type Primitive%20Component%20Object%20Reference) (OtherActor :type Actor%20Object%20Reference) (OtherComp :type Primitive%20Component%20Object%20Reference) (OtherBodyIndex :type Integer))
  (Variables|Default|SetOVERLAPPED_M false))

(event OnComponentBeginOverlap(Box_R1)
  (params (OverlappedComponent :type Primitive%20Component%20Object%20Reference) (OtherActor :type Actor%20Object%20Reference) (OtherComp :type Primitive%20Component%20Object%20Reference) (OtherBodyIndex :type Integer) (bFromSweep :type Boolean) (SweepResult :type Hit%20Result%20Structure%20%28by%20ref%29))
  (bind _output_get (Variables|Default|SetOverlapped%20Component%20OF%20R1 OverlappedComponent))
  (if (> (CallFunction|GetForwardSpeed) 4e+01)
    (if (not (== _output_get (Variables|Default|GetOverlapped%20Component%20OF%20L)))
      (Variables|Default|SetOVERLAPPED_S true)
      (Variables|Default|SetIS_RIGHT? true)
      (Utilities|FlowControl|Delay 0.5)
      (Variables|Default|SetOVERLAPPED_S false))))

(event Custom|AI_reset_loc
  (bind _astuning_car_game_inst (Utilities|Casting|CastToTuningCar_GameInst (Game|GetGameInstance)))
  (Variables|Default|SetRESPAWN_T (Variables|/Game/TuningCars/Blueprint/HUD/main_menu.main_menu_C|GetRACE_T (Variables|/Game/TuningCars/Blueprint/TuningCar_GameInst.TuningCar_GameInst_C|Getmain%20menu _astuning_car_game_inst)))
  (if (Variables|/Game/TuningCars/Blueprint/AliceGT/AliceGT.AliceGT_C|Getai__reset_location (Variables|/Game/TuningCars/Blueprint/HUD/main_menu.main_menu_C|Getcar (Variables|/Game/TuningCars/Blueprint/TuningCar_GameInst.TuningCar_GameInst_C|Getmain%20menu _astuning_car_game_inst)))
    (Transformation|SetActorTransform (Math|Transform|MakeTransform (- (.location (Variables|Default|GetRESPAWN_T)) "800.000000, 0, 0") (.rotation (Variables|Default|GetRESPAWN_T)) (.scale (Variables|Default|GetRESPAWN_T))) false true)))

(event Custom|CE_ResetDoOnceImpactSound
  ;[0.003424 0.3159 1 0.386] impact sounds
  ;;[1 1 1] CE Reset Do Once
  (Utilities|FlowControl|Delay 0.666)
  (Utilities|FlowControl|DoOnce false) ; enters at Reset
)

(event EventBeginPlay
  ;[0.0457 0.475 0] BeginPlay
  (Utilities|FlowControl|Sequence
    (:then_0
      (Utilities|AI)
      (CallFunction|AIResetLoc))
    (:then_1
      (Utilities|FlowControl|Delay 0.05)
      ;;[1 1 1] hide driver's mesh
      (Development|SetHiddeninGame (Variables|Default|GetDriver) true false))))

(event EventTick
  (params (DeltaSeconds :type Float%20%28single-precision%29))
  ;[0.0457 0.475 0] BeginPlay
  (Utilities|AI) ; enters at TICK
)

(fn ConstructionScript)

(fn CaliperRotation
  (params (left_side :type Boolean) (InSocketName :type Name) (caliper :type Scene%20Component%20Object%20Reference) (front :type Boolean))
  (bind _mesh (Variables|Character|GetMesh))
  (bind _returnvalue (Transformation|GetSocketTransform _mesh InSocketName "RTS_Component"))
  (bind (_location _rotation) (Math|Transform|BreakTransform _returnvalue))
  ;[1 1 1] left caliper initial rotation
  (if left_side
    (LocalVariables|Setroll 1.8e+02))
  ;[1 1 1] get bone location and rotation
  (LocalVariables|Setwheel_location _location)
  ;[1 1 1] yaw limits
  (bind _output_get (LocalVariables|Setwheel_yaw (.Yaw (Math|Rotator|BreakRotator _rotation))))
  (if (and (< _output_get 6e+01) (> _output_get -6e+01))
    _
    (else
      (LocalVariables|Setwheel_yaw (+ (LocalVariables|Getwheel_yaw) 1.8e+02))))
  ;[1 1 1] rear wheels don't yaw
  (if front
    _
    (else
      (LocalVariables|Setwheel_yaw 0.0)))
  ;[1 1 1] rotate calipers
  (Transformation|SetRelativeLocationAndRotation caliper (LocalVariables|Getwheel_location) (Math|Rotator|MakeRotator (LocalVariables|Getroll) 0.0 (LocalVariables|Getwheel_yaw)) false false)
  (return))

(fn MarkerRotation
  (params (marker :type Scene%20Component%20Object%20Reference) (rotation :type Float%20%28single-precision%29) (rot_multiplier :type Float%20%28single-precision%29))
  (Transformation|SetRelativeRotation marker (Math|Rotator|MakeRotator (- (* rotation rot_multiplier) 127.0) 3.0 0.0) false false))

(fn Lights
  (params (PositionLightsIn :type Boolean) (brakeLights :type Boolean) (ReverseLights :type Boolean))
  (Variables|lights|SetPositionLights PositionLightsIn)
  (Variables|lights|SetBrakeLights brakeLights)
  (Variables|lights|SetReverseLights ReverseLights)
  ;[1 1 1] set local material vars
  ;;[1 1 1] position lights
  (if (Variables|lights|GetPositionLights)
    (LocalVariables|SetrearPosLightMaterial (Variables|lights|Getrear_position_light_material_on))
    (LocalVariables|SetfrontPosLightMaterial (Variables|lights|Getfront_position_light_material_on))
    (else
      (LocalVariables|SetrearPosLightMaterial (Variables|lights|Getrear_position_light_material_off))
      (LocalVariables|SetfrontPosLightMaterial (Variables|lights|Getfront_position_light_material_off))))
  ;;[1 1 1] reverse lights
  (if ReverseLights
    (LocalVariables|SetreverseLightMaterial (Variables|lights|GetReverse_Light_Material_on))
    (else
      (LocalVariables|SetreverseLightMaterial (Variables|lights|GetReverse_Light_Material_off))))
  ;;[1 1 1] brake lights
  (if brakeLights
    (LocalVariables|SetbrakeLightMaterial (Variables|lights|GetBrake_Light_Material_on))
    (else
      (LocalVariables|SetbrakeLightMaterial (Variables|lights|GetBrake_Light_Material_off))))
  ;[1 1 1] materials
  ;;[1 1 1] rear pos
  (Rendering|Material|SetMaterial (Variables|Character|GetMesh) (Variables|lights|Getrear_position_light_id) (LocalVariables|GetrearPosLightMaterial))
  ;;[1 1 1] front pos
  (Rendering|Material|SetMaterial (Variables|Character|GetMesh) (Variables|lights|Getfront_position_light_id) (LocalVariables|GetfrontPosLightMaterial))
  ;;[1 1 1] brake
  (Rendering|Material|SetMaterial (Variables|Character|GetMesh) (Variables|lights|GetBrakeLightMaterialID) (LocalVariables|GetbrakeLightMaterial))
  ;;[1 1 1] reverse
  (Rendering|Material|SetMaterial (Variables|Character|GetMesh) (Variables|lights|GetReverseLightMaterialID) (LocalVariables|GetreverseLightMaterial))
  ;[1 1 1] lights
  ;;[1 1 1] position
  (Rendering|SetVisibility (Variables|Default|Getfront_light_L) (Variables|lights|GetPositionLights) false)
  ;;[1 1 1] brake lights
  (Rendering|SetVisibility (Variables|Default|GetBrakeLightL) brakeLights false)
  ;;[1 1 1] reverse lights
  (Rendering|SetVisibility (Variables|Default|GetReverseLightL) ReverseLights false)
  (return))

(fn CheckCharonDoorArea
  (params (Object :type Actor%20Object%20Reference) (canEnterCar :type Boolean) (nearLeftDoor :type Boolean) (possession :type Boolean))
  ;[1 1 1] for overlap events
  (if (Class|Pawn|IsControlled)
    ;[1 1 1] for possession events
    (if possession
      ;[1 1 1] cast to Third Person Char or VR Char (for texts)
      ;;[1 1 1] third person or VR char
      (bind _asbp_third_person_character (Utilities|Casting|CastToBP_ThirdPersonCharacter Object :!label _label)
        (:then
          ;;[1 0.1146 0.6587] set Specific Player Controller (MULTIPLAYER)
          (bind _asbp_dc_player_controller (Utilities|Casting|CastToBP_DC_PlayerController (Pawn|GetController _asbp_third_person_character))
            (:then
              (Variables|Default|Setdc_player_controller _asbp_dc_player_controller))
            (:CastFailed
              ;;;[1 0 0.8421] for the driving player
              (bind _asbp_dc_player_controller_2 (Utilities|Casting|CastToBP_DC_PlayerController (Pawn|GetController self)))
              (Variables|Default|Setdc_player_controller _asbp_dc_player_controller_2)))
          ;;[1 1 1] show enter car text
          (Default|CeShowHideText _asbp_third_person_character (not canEnterCar)))
        (:CastFailed
          (bind _asbp_vrcharacter (Utilities|Casting|CastToBP_VRCharacter Object))
          (bind _asbp_dc_player_controller_3 (Utilities|Casting|CastToBP_DC_PlayerController (Pawn|GetController _asbp_vrcharacter)))
          (Variables|Default|Setdc_player_controller _asbp_dc_player_controller_3)
          (Default|ShowHideText _asbp_vrcharacter (not canEnterCar))))
      ;[1 1 1] set vars on DC Player Controller
      (Variables|/Game/DriveableCar_basic/Blueprints/BP_DC_PlayerController.BP_DC_PlayerController_C|SetCanEnterCar (Variables|Default|Getdc_player_controller) canEnterCar)
      (Variables|/Game/DriveableCar_basic/Blueprints/BP_DC_PlayerController.BP_DC_PlayerController_C|SetLeftDoor (Variables|Default|Getdc_player_controller) nearLeftDoor)
      (Variables|/Game/DriveableCar_basic/Blueprints/BP_DC_PlayerController.BP_DC_PlayerController_C|SetCarReference (Variables|Default|Getdc_player_controller) self)
      (return))
    (else
      (goto _label))))

(fn OnRepRearPositionLightMaterialon)

(fn OnRepFrontPositionLightMaterialon)

(fn OnRepThrottle)

(fn GetForwardSpeed
  (return (* (Class|WheeledVehicleMovementComponent|GetForwardSpeed (Variables|Default|GetVehicleMovement)) 0.036)))

(fn GETLANEINDEX
  (bind _outactors (Actor|GetAllActorsOfClass "/Game/TuningCars/Blueprint/AI_CAR/ROAD.ROAD_C"))
  (for _array_element _outactors
    (if (Utilities|Enum|Equal(Enum) (Variables|/Game/TuningCars/Blueprint/AI_CAR/ROAD.ROAD_C|GetLANE_TYPE _array_element) (Variables|Default|GetLANE%20TYPE))
      (bind _output_get (Variables|Default|SetROAD _array_element))
      (bind _output_get_2 (Variables|Default|Setmax_speed (Variables|/Game/TuningCars/Blueprint/AI_CAR/ROAD.ROAD_C|GetSPEED%20LIMIT _output_get)))
      (return _output_get_2))))

(fn GETLANE
  (params (SPLINE :type Spline%20Component%20Object%20Reference))
  (bind _returnvalue (Transformation|GetActorLocation))
  (bind _returnvalue_2 (Class|SplineComponent|FindTangentClosesttoWorldLocation SPLINE _returnvalue "World"))
  (bind _returnvalue_3 (Math|Vector|Normalize _returnvalue_2))
  (bind _returnvalue_4 (* _returnvalue_3 0.0))
  (bind _returnvalue_5 (+ _returnvalue_4 _returnvalue))
  (bind _returnvalue_6 (Spline|FindLocationClosesttoWorldLocation SPLINE _returnvalue_5 "World"))
  (Utilities|IsValid SPLINE
    (:Is%20Valid
      (Rendering|Debug|DrawDebugSphere (Math|Vector|VectorGetAbs _returnvalue_2) 1e+02 12 "(R=1.000000,G=1.000000,B=1.000000,A=1.000000)" 0.0)
      (Rendering|Debug|DrawDebugSphere _returnvalue_6 1e+02 12 "(R=1.000000,G=0.074850,B=0.194583,A=1.000000)" 0.0)
      (return (Math|Float|MapRangeClamped (.yaw (Math|Rotator|Delta(Rotator) (Math|Rotator|FindLookatRotation _returnvalue _returnvalue_6) (Transformation|GetActorRotation))) 0.0 0.0 0.0 0.0)))))

(fn SetCarTransform
  (params (NewTransform :type Transform%20%28by%20ref%29))
  (Transformation|SetWorldTransform (Variables|/Script/Engine.MovementComponent|GetUpdatedPrimitive (Variables|Default|GetVehicleMovement)) NewTransform false true))