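; AI-driven car that follows the spline of a ROAD actor found on BeginPlay.
; Each tick it steers toward a spline point ahead and scales throttle by the steering value.
; Sharp steering reverses throttle, inverts steering and triggers a timed handbrake once until the turn eases.
; It prints driving values and draws a debug sphere at the target point each frame.
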(event EventBeginPlay
  (|CallParentFunction)
  (bind _returnvalue (Actor|GetActorOfClass "/Game/TuningCars/Blueprint/AI_CAR/ROAD.ROAD_C"))
  (Variables|Default|SetRoad%20Line (Variables|/Game/TuningCars/Blueprint/AI_CAR/ROAD.ROAD_C|GetSpline _returnvalue)))

(event EventTick
  (params (DeltaSeconds :type Float%20%28single-precision%29))
  (bind _returnvalue (Transformation|GetActorLocation))
  ;[1 1 1] AI Driving Logic
  (Utilities|FlowControl|Sequence
    (:then_0
      (bind _road_line (Variables|Default|GetRoad%20Line)
        (:then
          ;;[1 1 1] Steering
          (bind _output_get (Variables|Default|SetNext%20Location (.Next%20Location (CallFunction|GetNextLocationonASpline _road_line _returnvalue 2e+03))))
          (bind _output_get_2 (Variables|Default|SetSteering%20Value (CallFunction|GetSteeringtoLocation _returnvalue _output_get (Transformation|GetActorRotation))))
          (bind _output_get_3 (Variables|Default|SetBackward%20Direction (or (< (Variables|Default|GetSteering%20Value) -0.7) (> (Variables|Default|GetSteering%20Value) 0.7))))
          (Variables|Default|SetThrottle%20Value (select _output_get_3 (* -1 (Math|Float|MapRangeClamped _output_get_2 0.0 1.0 0.8 0.2)) (Math|Float|MapRangeClamped _output_get_2 0.0 1.0 0.8 0.2))))
        (:else)))
    (:then_1
      ;;[1 1 1] Throttle and Steering
      (CallFunction|AISteering (select (< (Variables|Default|GetThrottle%20Value) 0.0) (* -1 (Variables|Default|GetSteering%20Value)) (Variables|Default|GetSteering%20Value)))
      (CallFunction|AIThrottle (Variables|Default|GetThrottle%20Value))
      (if (Variables|Default|GetBackward%20Direction)
        ;;[1 1 1] HandBrake
        (Utilities|FlowControl|DoOnce false :!label _label
          (:Completed
            (CallFunction|AIHandBrake true)
            (Utilities|FlowControl|Delay 2.0)
            (CallFunction|AIHandBrake false)))
        (else
          (goto _label Reset))))
    (:then_2
      ;;[1 1 1] Debugging
      (Development|PrintString (Utilities|String|ToString(Text) (Utilities|Text|FormatText "Throttle Value: {Throttle} 
Steering Value: {Steering} 
Next Spline Point Location: {Next Location}" (Variables|Default|GetSteering%20Value) (Variables|Default|GetThrottle%20Value) (Utilities|Text|ToText(String) (Variables|Default|GetNext%20Location)))) true true "(R=0.000000,G=0.660000,B=1.000000,A=1.000000)" 0.0)
      (Collision|SphereTraceByChannel (Variables|Default|GetNext%20Location) (Variables|Default|GetNext%20Location) 1e+02 "TraceTypeQuery1" false 0 "ForOneFrame"))))

(fn ConstructionScript
  (|CallParentFunction))