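; Blueprint function library of helpers for AI vehicles that follow a spline path.
; GetNextLocationOnASpline steps a given distance along the tangent nearest the current location, snaps that point back onto the spline, and returns it with its 2D distance.
; GetSteeringToLocation converts the yaw difference between the current rotation and the look-at rotation toward a wanted location into a clamped, normalized steering value.
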(fn GetNextLocationonASpline
  (params (Spline :type Spline%20Component%20Object%20Reference) (Current%20Location :type Vector) (Forward%20Distance :type Float%20%28single-precision%29))
  (bind _returnvalue (Class|SplineComponent|FindTangentClosesttoWorldLocation Spline Current%20Location "World"))
  (bind _returnvalue_2 (Math|Vector|Normalize _returnvalue))
  (bind _returnvalue_3 (* _returnvalue_2 Forward%20Distance))
  (bind _returnvalue_4 (+ _returnvalue_3 Current%20Location))
  (bind _returnvalue_5 (Spline|FindLocationClosesttoWorldLocation Spline _returnvalue_4 "World"))
  ;[1 1 1] Get Next Location on a Spline, Based on the Current Location
  (return _returnvalue_5 (Math|Vector|Distance2D(Vector) _returnvalue_5 Current%20Location)))

(fn GetSteeringtoLocation
  (params (Current%20Location :type Vector) (Wanted%20Location :type Vector) (Current%20Rotation :type Rotator))
  ;[1 1 1] Get Steering to Location
  (return (Math|Float|MapRangeClamped (.yaw (Math|Rotator|Delta(Rotator) (Math|Rotator|FindLookatRotation Current%20Location Wanted%20Location) Current%20Rotation)) -9e+01 9e+01 -1.0 1.0)))