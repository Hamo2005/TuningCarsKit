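; 3D tuning menu for the car customization screen, with clickable part icons that glow and pulse on hover via dynamic materials and a timeline.
; Clicking an icon calls SetTuning, which moves the spring-arm camera to a car socket, toggles the icons and feeds GameInstance part lists to the MenuTuning widget.
; Space toggles free-look, hiding the icons for mouse orbit with a pitch check; the wheel adjusts zoom.
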(event OnBeginCursorOver(tuning)
  (params (TouchedComponent :type Primitive%20Component%20Object%20Reference))
  ;[1 1 1] over tuning
  (Utilities|OverEffect3D TouchedComponent (Variables|Default|Gettuning_mat))
  ;[1 1 1] resize icon 3D
  (bind _scale (Timeline|resize%20icons%203D PlayFromStart)
    (:Update
      (Transformation|SetRelativeScale3D (Variables|Default|GethoverComp) _scale))))

(event OnEndCursorOver(tuning)
  (params (TouchedComponent :type Primitive%20Component%20Object%20Reference))
  ;[1 1 1] end over tuning
  (Utilities|EndOverEffect3D TouchedComponent (Variables|Default|Gettuning_mat))
  ;[1 1 1] set original size of icon 3D
  (Transformation|SetRelativeScale3D (Variables|Default|GethoverComp) "1.000000,1.000000,1.000000")
  ;[1 1 1] resize icon 3D
  (bind _scale (Timeline|resize%20icons%203D Stop)
    (:Update
      (Transformation|SetRelativeScale3D (Variables|Default|GethoverComp) _scale))))

(event OnClicked(hood)
  (params (TouchedComponent :type Primitive%20Component%20Object%20Reference) (ButtonPressed :type Key%20Structure :default "None"))
  ;[1 1 1] show hood menu
  (Variables|/Game/TuningCars/Blueprint/HUD/menu_tuning.menu_tuning_C|SetcurrItemName (Variables|Default|GetmenuTuning) "hood")
  (CallFunction|SetTuning 4.3e-05 -26.42585 -179.908386 4.2e+02 false (Variables|/Game/TuningCars/Blueprint/TuningCar_GameInst.TuningCar_GameInst_C|Gethoods (Variables|Default|GetgameInst)) "Vehicle_Base"))

(event OnClicked(glass_f)
  (params (TouchedComponent :type Primitive%20Component%20Object%20Reference) (ButtonPressed :type Key%20Structure :default "None"))
  ;[1 1 1] show glass_f menu
  (Variables|/Game/TuningCars/Blueprint/HUD/menu_tuning.menu_tuning_C|SetcurrItemName (Variables|Default|GetmenuTuning) "glass_f")
  (CallFunction|SetTuning 4.3e-05 -18.52692 154.88089 4e+02 false (Variables|/Game/TuningCars/Blueprint/TuningCar_GameInst.TuningCar_GameInst_C|Getglass_f (Variables|Default|GetgameInst)) "Vehicle_Base"))

(event OnClicked(glass_b)
  (params (TouchedComponent :type Primitive%20Component%20Object%20Reference) (ButtonPressed :type Key%20Structure :default "None"))
  ;[1 1 1] show glass_b menu
  (Variables|/Game/TuningCars/Blueprint/HUD/menu_tuning.menu_tuning_C|SetcurrItemName (Variables|Default|GetmenuTuning) "glass_b")
  (CallFunction|SetTuning -7.6e-05 -19.32233 20.593683 3.7e+02 false (Variables|/Game/TuningCars/Blueprint/TuningCar_GameInst.TuningCar_GameInst_C|Getglass_b (Variables|Default|GetgameInst)) "Vehicle_Base"))

(event OnClicked(tuning)
  (params (TouchedComponent :type Primitive%20Component%20Object%20Reference) (ButtonPressed :type Key%20Structure :default "None"))
  ;[1 1 1] Show car body menu
  (Variables|/Game/TuningCars/Blueprint/HUD/menu_tuning.menu_tuning_C|SetcurrItemName (Variables|Default|GetmenuTuning) "body")
  (CallFunction|SetTuning -1e+01 -15.0 9e+01 4.4e+02 (not (Variables|/Script/Engine.SceneComponent|GetbVisible (Variables|Default|Getwheel))) (Variables|/Game/TuningCars/Blueprint/TuningCar_GameInst.TuningCar_GameInst_C|Gettexture (Variables|Default|GetgameInst)) "Vehicle_Base")
  (Utilities|Casting|CastToTuningCar_GameInst (Game|GetGameInstance))
  (Widget|SetVisibility (Variables|/Game/TuningCars/Blueprint/HUD/menu_tuning.menu_tuning_C|GetABILITY_B (Variables|Default|GetmenuTuning)) "SelfHitTestInvisible"))

(event OnClicked(molding)
  (params (TouchedComponent :type Primitive%20Component%20Object%20Reference) (ButtonPressed :type Key%20Structure :default "None"))
  ;[1 1 1] show molding menu
  (Variables|/Game/TuningCars/Blueprint/HUD/menu_tuning.menu_tuning_C|SetcurrItemName (Variables|Default|GetmenuTuning) "side")
  (CallFunction|SetTuning -7e-06 -11.403075 74.786766 2.7e+02 false (Variables|/Game/TuningCars/Blueprint/TuningCar_GameInst.TuningCar_GameInst_C|Getmoldings (Variables|Default|GetgameInst)) "Vehicle_Base"))

(event OnBeginCursorOver(wheel)
  (params (TouchedComponent :type Primitive%20Component%20Object%20Reference))
  ;[1 1 1] over wheel
  (Utilities|OverEffect3D TouchedComponent (Variables|Default|Getwheel_mat))
  ;[1 1 1] resize icon 3D
  (bind _scale (Timeline|resize%20icons%203D PlayFromStart)
    (:Update
      (Transformation|SetRelativeScale3D (Variables|Default|GethoverComp) _scale))))

(event OnBeginCursorOver(hood)
  (params (TouchedComponent :type Primitive%20Component%20Object%20Reference))
  ;[1 1 1] over hood
  (Utilities|OverEffect3D TouchedComponent (Variables|Default|Gethood_mat))
  ;[1 1 1] resize icon 3D
  (bind _scale (Timeline|resize%20icons%203D PlayFromStart)
    (:Update
      (Transformation|SetRelativeScale3D (Variables|Default|GethoverComp) _scale))))

(event OnBeginCursorOver(molding)
  (params (TouchedComponent :type Primitive%20Component%20Object%20Reference))
  ;[1 1 1] over molding
  (Utilities|OverEffect3D TouchedComponent (Variables|Default|Getmolding_mat))
  ;[1 1 1] resize icon 3D
  (bind _scale (Timeline|resize%20icons%203D PlayFromStart)
    (:Update
      (Transformation|SetRelativeScale3D (Variables|Default|GethoverComp) _scale))))

(event OnClicked(bumper_b)
  (params (TouchedComponent :type Primitive%20Component%20Object%20Reference) (ButtonPressed :type Key%20Structure :default "None"))
  ;[1 1 1] show bumper_b menu
  (Variables|/Game/TuningCars/Blueprint/HUD/menu_tuning.menu_tuning_C|SetcurrItemName (Variables|Default|GetmenuTuning) "bumper_b")
  (CallFunction|SetTuning -5.8e-05 -12.4851826 6.667822 4e+02 false (Variables|/Game/TuningCars/Blueprint/TuningCar_GameInst.TuningCar_GameInst_C|Getbumpers_down (Variables|Default|GetgameInst)) "Vehicle_Base"))

(event OnBeginCursorOver(bumper_b)
  (params (TouchedComponent :type Primitive%20Component%20Object%20Reference))
  ;[1 1 1] over bumper_b
  (Utilities|OverEffect3D TouchedComponent (Variables|Default|Getbumper_b_mat))
  ;[1 1 1] resize icon 3D
  (bind _scale (Timeline|resize%20icons%203D PlayFromStart)
    (:Update
      (Transformation|SetRelativeScale3D (Variables|Default|GethoverComp) _scale))))

(event OnClicked(spoler)
  (params (TouchedComponent :type Primitive%20Component%20Object%20Reference) (ButtonPressed :type Key%20Structure :default "None"))
  ;[1 1 1] show spoler menu
  (Variables|/Game/TuningCars/Blueprint/HUD/menu_tuning.menu_tuning_C|SetcurrItemName (Variables|Default|GetmenuTuning) "spoler")
  (CallFunction|SetTuning -0.327463 -23.795353 151.120575 2e+02 false (Variables|/Game/TuningCars/Blueprint/TuningCar_GameInst.TuningCar_GameInst_C|Getspolers (Variables|Default|GetgameInst)) "spoilersocet"))

(event OnBeginCursorOver(spoler)
  (params (TouchedComponent :type Primitive%20Component%20Object%20Reference))
  ;[1 1 1] over spoler
  (Utilities|OverEffect3D TouchedComponent (Variables|Default|Getspoler_mat))
  ;[1 1 1] resize icon 3D
  (bind _scale (Timeline|resize%20icons%203D PlayFromStart)
    (:Update
      (Transformation|SetRelativeScale3D (Variables|Default|GethoverComp) _scale))))

(event OnBeginCursorOver(bumper_f)
  (params (TouchedComponent :type Primitive%20Component%20Object%20Reference))
  ;[1 1 1] over bumper_f
  (Utilities|OverEffect3D TouchedComponent (Variables|Default|Getbumper_f_mat))
  ;[1 1 1] resize icon 3D
  (bind _scale (Timeline|resize%20icons%203D PlayFromStart)
    (:Update
      (Transformation|SetRelativeScale3D (Variables|Default|GethoverComp) _scale))))

(event OnBeginCursorOver(glass_f)
  (params (TouchedComponent :type Primitive%20Component%20Object%20Reference))
  ;[1 1 1] over glass_f
  (Utilities|OverEffect3D TouchedComponent (Variables|Default|Getglass_f_mat))
  ;[1 1 1] resize icon 3D
  (bind _scale (Timeline|resize%20icons%203D PlayFromStart)
    (:Update
      (Transformation|SetRelativeScale3D (Variables|Default|GethoverComp) _scale))))

(event OnEndCursorOver(wheel)
  (params (TouchedComponent :type Primitive%20Component%20Object%20Reference))
  ;[1 1 1] end over wheel
  (Utilities|EndOverEffect3D TouchedComponent (Variables|Default|Getwheel_mat))
  ;[1 1 1] set original size of icon 3D
  (Transformation|SetRelativeScale3D (Variables|Default|GethoverComp) "1.000000,1.000000,1.000000")
  ;[1 1 1] resize icon 3D
  (bind _scale (Timeline|resize%20icons%203D Stop)
    (:Update
      (Transformation|SetRelativeScale3D (Variables|Default|GethoverComp) _scale))))

(event OnClicked(bumper_f)
  (params (TouchedComponent :type Primitive%20Component%20Object%20Reference) (ButtonPressed :type Key%20Structure :default "None"))
  ;[1 1 1] show bumper_f menu
  (Variables|/Game/TuningCars/Blueprint/HUD/menu_tuning.menu_tuning_C|SetcurrItemName (Variables|Default|GetmenuTuning) "bumper_f")
  (CallFunction|SetTuning 4.7e-05 -10.927059 177.863113 3.9e+02 false (Variables|/Game/TuningCars/Blueprint/TuningCar_GameInst.TuningCar_GameInst_C|Getbumpers (Variables|Default|GetgameInst)) "Vehicle_Base"))

(event OnEndCursorOver(hood)
  (params (TouchedComponent :type Primitive%20Component%20Object%20Reference))
  ;[1 1 1] end over hood
  (Utilities|EndOverEffect3D TouchedComponent (Variables|Default|Gethood_mat))
  ;[1 1 1] set original size of icon 3D
  (Transformation|SetRelativeScale3D (Variables|Default|GethoverComp) "1.000000,1.000000,1.000000")
  ;[1 1 1] resize icon 3D
  (bind _scale (Timeline|resize%20icons%203D Stop)
    (:Update
      (Transformation|SetRelativeScale3D (Variables|Default|GethoverComp) _scale))))

(event OnEndCursorOver(molding)
  (params (TouchedComponent :type Primitive%20Component%20Object%20Reference))
  ;[1 1 1] end over molding
  (Utilities|EndOverEffect3D TouchedComponent (Variables|Default|Getmolding_mat))
  ;[1 1 1] set original size of icon 3D
  (Transformation|SetRelativeScale3D (Variables|Default|GethoverComp) "1.000000,1.000000,1.000000")
  ;[1 1 1] resize icon 3D
  (bind _scale (Timeline|resize%20icons%203D Stop)
    (:Update
      (Transformation|SetRelativeScale3D (Variables|Default|GethoverComp) _scale))))

(event OnEndCursorOver(bumper_b)
  (params (TouchedComponent :type Primitive%20Component%20Object%20Reference))
  ;[1 1 1] end over bumper_b
  (Utilities|EndOverEffect3D TouchedComponent (Variables|Default|Getbumper_b_mat))
  ;[1 1 1] set original size of icon 3D
  (Transformation|SetRelativeScale3D (Variables|Default|GethoverComp) "1.000000,1.000000,1.000000")
  ;[1 1 1] resize icon 3D
  (bind _scale (Timeline|resize%20icons%203D Stop)
    (:Update
      (Transformation|SetRelativeScale3D (Variables|Default|GethoverComp) _scale))))

(event OnEndCursorOver(spoler)
  (params (TouchedComponent :type Primitive%20Component%20Object%20Reference))
  ;[1 1 1] end over spoler
  (Utilities|EndOverEffect3D TouchedComponent (Variables|Default|Getspoler_mat))
  ;[1 1 1] set original size of icon 3D
  (Transformation|SetRelativeScale3D (Variables|Default|GethoverComp) "1.000000,1.000000,1.000000")
  ;[1 1 1] resize icon 3D
  (bind _scale (Timeline|resize%20icons%203D Stop)
    (:Update
      (Transformation|SetRelativeScale3D (Variables|Default|GethoverComp) _scale))))

(event OnEndCursorOver(bumper_f)
  (params (TouchedComponent :type Primitive%20Component%20Object%20Reference))
  ;[1 1 1] end over bumper_f
  (Utilities|EndOverEffect3D TouchedComponent (Variables|Default|Getbumper_f_mat))
  ;[1 1 1] set original size of icon 3D
  (Transformation|SetRelativeScale3D (Variables|Default|GethoverComp) "1.000000,1.000000,1.000000")
  ;[1 1 1] resize icon 3D
  (bind _scale (Timeline|resize%20icons%203D Stop)
    (:Update
      (Transformation|SetRelativeScale3D (Variables|Default|GethoverComp) _scale))))

(event OnEndCursorOver(glass_f)
  (params (TouchedComponent :type Primitive%20Component%20Object%20Reference))
  ;[1 1 1] end over glass_f
  (Utilities|EndOverEffect3D TouchedComponent (Variables|Default|Getglass_f_mat))
  ;[1 1 1] set original size of icon 3D
  (Transformation|SetRelativeScale3D (Variables|Default|GethoverComp) "1.000000,1.000000,1.000000")
  ;[1 1 1] resize icon 3D
  (bind _scale (Timeline|resize%20icons%203D Stop)
    (:Update
      (Transformation|SetRelativeScale3D (Variables|Default|GethoverComp) _scale))))

(event OnClicked(wheel)
  (params (TouchedComponent :type Primitive%20Component%20Object%20Reference) (ButtonPressed :type Key%20Structure :default "None"))
  ;[1 1 1] show wheel menu
  (Variables|/Game/TuningCars/Blueprint/HUD/menu_tuning.menu_tuning_C|SetcurrItemName (Variables|Default|GetmenuTuning) "wheel")
  (CallFunction|SetTuning -6.1e-05 -3.931901 94.883316 1.1e+02 false (Variables|/Game/TuningCars/Blueprint/TuningCar_GameInst.TuningCar_GameInst_C|Getwheels (Variables|Default|GetgameInst)) "Wheel_Front_Left"))

(event OnBeginCursorOver(glass_b)
  (params (TouchedComponent :type Primitive%20Component%20Object%20Reference))
  ;[1 1 1] over glass_b
  (Utilities|OverEffect3D TouchedComponent (Variables|Default|Getglass_b_mat))
  ;[1 1 1] resize icon 3D
  (bind _scale (Timeline|resize%20icons%203D PlayFromStart)
    (:Update
      (Transformation|SetRelativeScale3D (Variables|Default|GethoverComp) _scale))))

(event OnEndCursorOver(glass_b)
  (params (TouchedComponent :type Primitive%20Component%20Object%20Reference))
  ;[1 1 1] end over glass_b
  (Utilities|EndOverEffect3D TouchedComponent (Variables|Default|Getglass_b_mat))
  ;[1 1 1] set original size of icon 3D
  (Transformation|SetRelativeScale3D (Variables|Default|GethoverComp) "1.000000,1.000000,1.000000")
  ;[1 1 1] resize icon 3D
  (bind _scale (Timeline|resize%20icons%203D Stop)
    (:Update
      (Transformation|SetRelativeScale3D (Variables|Default|GethoverComp) _scale))))

(event EventEndPlay
  (params (EndPlayReason :type EEndPlayReason%20Enum :default "Destroyed"))
  ;[1 1 1] stop embient sound in EndPlay Event
  (Audio|Components|Audio|Stop (Variables|Default|Gettuning_embient_Cue)))

(event EventBeginPlay
  ;[1 1 1] play embient sound in BeginPlay Event
  (Audio|Components|Audio|Play (Variables|Default|Gettuning_embient_Cue) 0.0)
  ;[1 1 1] get references: car mesh, game instance, menu tuning
  (bind _astuning_car_game_inst (Utilities|Casting|CastToTuningCar_GameInst (Game|GetGameInstance)))
  (bind _output_get (Variables|Default|SetgameInst _astuning_car_game_inst))
  (Variables|Default|SetmenuTuning (Variables|/Game/TuningCars/Blueprint/TuningCar_GameInst.TuningCar_GameInst_C|Getmenu_tuning _output_get))
  (Variables|Default|SetcarMesh (Variables|/Script/PhysXVehicles.WheeledVehicle|GetMesh (Variables|/Game/TuningCars/Blueprint/TuningCar_GameInst.TuningCar_GameInst_C|Getcar _astuning_car_game_inst))))

(event Input|MouseEvents|MouseX
  (params (AxisValue :type Float%20%28single-precision%29))
  ;[1 1 1] Camera Rotate X
  (if (Variables|Default|GetisFreeLook)
    (Transformation|AddWorldRotation (Variables|Default|GetmenuRotate) (Math|Rotator|MakeRotator 0.0 0.0 AxisValue) false false)))

(event Input|MouseEvents|MouseY
  (params (AxisValue :type Float%20%28single-precision%29))
  ;[1 1 1] Camera Rotate Y
  (if (Variables|Default|GetisFreeLook)
    (Utilities|CameraBlockFloor AxisValue
      (:True
        (Transformation|AddLocalRotation (Variables|Default|GetmenuRotate) (Math|Rotator|MakeRotator 0.0 AxisValue 0.0) false false)))))

(event Input|MouseEvents|MouseWheelAxis
  (params (AxisValue :type Float%20%28single-precision%29))
  ;[1 1 1] Set Camera Arm Length by Mouse Wheel
  (Variables|/Script/Engine.SpringArmComponent|SetTargetArmLength (Variables|Default|GetmenuRotate) (+ (Variables|/Script/Engine.SpringArmComponent|GetTargetArmLength (Variables|Default|GetmenuRotate)) (* AxisValue -1e+01))))

(event Input|KeyboardEvents|SpaceBar
  (params (Key :type Key%20Structure :default "None"))
  ;[1 1 1] set free look
  (:Released
    (CallFunction|SetFreeLook)))

(fn ConstructionScript
  (bind _returnvalue (Rendering|Material|CreateDynamicMaterialInstance (Variables|Default|Gettuning) 0 "/Game/TuningCars/Materials/HUD/tuningmenu_Inst.tuningmenu_Inst" "None" :!class /Script/Engine.PrimitiveComponent))
  (Variables|Default|Settuning_mat _returnvalue)
  (bind _returnvalue_2 (Rendering|Material|CreateDynamicMaterialInstance (Variables|Default|Getwheel) 0 "/Game/TuningCars/Materials/HUD/Disc_M_Inst.Disc_M_Inst" "None" :!class /Script/Engine.PrimitiveComponent))
  (Variables|Default|Setwheel_mat _returnvalue_2)
  (bind _returnvalue_3 (Rendering|Material|CreateDynamicMaterialInstance (Variables|Default|Gethood) 0 "/Game/TuningCars/Materials/HUD/kapot_M_Inst.kapot_M_Inst" "None" :!class /Script/Engine.PrimitiveComponent))
  (Variables|Default|Sethood_mat _returnvalue_3)
  (bind _returnvalue_4 (Rendering|Material|CreateDynamicMaterialInstance (Variables|Default|Getbumper_b) 0 "/Game/TuningCars/Materials/HUD/bumperdown_M_Inst.bumperdown_M_Inst" "None" :!class /Script/Engine.PrimitiveComponent))
  (Variables|Default|Setbumper_b_mat _returnvalue_4)
  (bind _returnvalue_5 (Rendering|Material|CreateDynamicMaterialInstance (Variables|Default|Getspoler) 0 "/Game/TuningCars/Materials/HUD/spoiler_M_Inst.spoiler_M_Inst" "None" :!class /Script/Engine.PrimitiveComponent))
  (Variables|Default|Setspoler_mat _returnvalue_5)
  (bind _returnvalue_6 (Rendering|Material|CreateDynamicMaterialInstance (Variables|Default|Getbumper_f) 0 "/Game/TuningCars/Materials/HUD/bumperUp_M_Inst.bumperUp_M_Inst" "None" :!class /Script/Engine.PrimitiveComponent))
  (Variables|Default|Setbumper_f_mat _returnvalue_6)
  (bind _returnvalue_7 (Rendering|Material|CreateDynamicMaterialInstance (Variables|Default|Getglass_f) 0 "/Game/TuningCars/Materials/HUD/glassUP_M_Inst.glassUP_M_Inst" "None" :!class /Script/Engine.PrimitiveComponent))
  (Variables|Default|Setglass_f_mat _returnvalue_7)
  (bind _returnvalue_8 (Rendering|Material|CreateDynamicMaterialInstance (Variables|Default|Getglass_b) 0 "/Game/TuningCars/Materials/HUD/glassdown_M_Inst.glassdown_M_Inst" "None" :!class /Script/Engine.PrimitiveComponent))
  (Variables|Default|Setglass_b_mat _returnvalue_8)
  (bind _returnvalue_9 (Rendering|Material|CreateDynamicMaterialInstance (Variables|Default|Getmolding) 0 "/Game/TuningCars/Materials/HUD/modling_M_Inst.modling_M_Inst" "None" :!class /Script/Engine.PrimitiveComponent))
  (Variables|Default|Setmolding_mat _returnvalue_9))

(fn SetTuning
  (params (X%20%28Roll%29 :type Float%20%28single-precision%29) (Y%20%28Pitch%29 :type Float%20%28single-precision%29) (Z%20%28Yaw%29 :type Float%20%28single-precision%29) (TargetArmLength :type Float%20%28single-precision%29) (bNewVisibility :type Boolean) (item :type Array%20of%20Tuning%20Item%20Structures) (InSocketName :type Name))
  (bind _returnvalue (Game|GetPlayerController 0))
  (bind _menutuning (Variables|Default|GetmenuTuning))
  (bind _menurotate (Variables|Default|GetmenuRotate))
  (bind _menutuning_2 (Variables|Default|GetmenuTuning))
  (bind _panelcolor (Variables|/Game/TuningCars/Blueprint/HUD/menu_tuning.menu_tuning_C|GetpanelColor _menutuning))
  ;[1 1 1] Set camera Parameters
  (Transformation|SetRelativeRotation _menurotate (Math|Rotator|MakeRotator X%20%28Roll%29 Y%20%28Pitch%29 Z%20%28Yaw%29) false false)
  (Variables|/Script/Engine.SpringArmComponent|SetTargetArmLength _menurotate TargetArmLength)
  (LocalVariables|Setnew%20Visible bNewVisibility)
  (Transformation|SetWorldLocation (Variables|Default|GetmenuRotate) (Transformation|GetSocketLocation (Variables|Default|GetcarMesh) InSocketName) false false)
  ;[1 1 1] Clear array of current materials
  (Utilities|Array|Clear (Variables|/Game/TuningCars/Blueprint/AliceGT/AliceGT.AliceGT_C|Getcurrent%20mats (Variables|/Game/TuningCars/Blueprint/TuningCar_GameInst.TuningCar_GameInst_C|Getcar (Variables|Default|GetgameInst))))
  ;[1 1 1] play sound of camera moving
  (Audio|PlaySound2D "/Game/TuningCars/Sounds/Wav/whoos.whoos" 1.0 1.0 0.0 0 0)
  ;[1 1 1] hide/show menu/widgets
  (Rendering|SetVisibility (Variables|Default|Getwheel) (LocalVariables|Getnew%20Visible) false)
  (if (LocalVariables|Getnew%20Visible)
    (Widget|SetVisibility _menutuning_2 "Hidden")
    (Variables|/Script/Engine.PlayerController|SetbEnableClickEvents _returnvalue true)
    (Widget|SetVisibility _panelcolor "SelfHitTestInvisible")
    (else
      (Default|SetItems _menutuning_2 item)
      (Variables|/Script/Engine.PlayerController|SetbEnableClickEvents _returnvalue false)
      (if (Variables|Default|GetisFreeLook)
        (Widget|SetVisibility _panelcolor "Hidden")))))

(fn SetFreeLook
  ;[1 1 1] if
  (if (Variables|Default|GetisFreeLook)
    ;[1 1 1] show mouse cursor
    (bind _asvehicle_player_controller (Utilities|Casting|CastToVehiclePlayerController (Game|GetPlayerController 0)))
    (Variables|/Script/Engine.PlayerController|SetbShowMouseCursor _asvehicle_player_controller true)
    ;[1 1 1] show tuning menu3D
    (Variables|Default|SetisFreeLook false)
    (CallFunction|SetTuning -9.891506 -18.335089 128.417267 4.4e+02 true (Variables|Default|GetnullItem) "None")
    (else
      ;[1 1 1] show mouse cursor
      (bind _asvehicle_player_controller_2 (Utilities|Casting|CastToVehiclePlayerController (Game|GetPlayerController 0)))
      (Variables|/Script/Engine.PlayerController|SetbShowMouseCursor _asvehicle_player_controller_2 false)
      ;[1 1 1] hide tuning menu3D
      (Variables|Default|SetisFreeLook true)
      (CallFunction|SetTuning 0.0 -18.335089 128.417267 4.4e+02 false (Variables|Default|GetnullItem) "None"))))